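; Player controller Blueprint that handles worker selection and building placement input.
; On BeginPlay it caches HUD_BP and adds the main HUD widget, passing it the BuildingManager.
; Selection events start and stop the HUD's selection, then append its returned WorkerUnit actors to WorkersSelected without duplicates and without clearing earlier picks.
; Left mouse confirms a build through BuildingManager, while Escape or Backspace cancels placement.
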(event `self.ReceiveBeginPlay`
  (bind _ashud_bp (cast `/Game/Blueprints/HUD_BP` (`PlayerController.GetHUD` (`GameplayStatics.GetPlayerController` 0))))
  (set `self.HUD` _ashud_bp)
  (bind _returnvalue (`|CreateWidget` "/Game/Blueprints/Main_HUD_BP.Main_HUD_BP_C" null self))
  (`UserWidget.AddToViewport` _returnvalue 0)
  (set `/Game/Blueprints/Main_HUD_BP.BuildingManager` (`self.BuildingManager`) _returnvalue)
  (`self.SetActorTickEnabled` true))

(event `self.OnStartSelection`
  (bind _hud (`self.HUD`))
  (`/Game/Blueprints/HUD_BP.StartSelection` _hud)
  (`KismetArrayLibrary.Array_Clear` (`/Game/Blueprints/HUD_BP.Out Actors` _hud)))

(event `self.OnEndSelection`
  (bind _hud (`self.HUD`))
  (bind _workersselected (`self.WorkersSelected`))
  (`/Game/Blueprints/HUD_BP.StopSelection` _hud)
  (for _array_element (`/Game/Blueprints/HUD_BP.Out Actors` _hud)
    (bind _asworker_unit (cast `WorkerUnit` _array_element))
    (if (`KismetArrayLibrary.Array_Contains` _workersselected _asworker_unit)
      (`KismetSystemLibrary.PrintString` "FoundActorAlreadyInWorers")
      (else
        (`KismetArrayLibrary.Array_Add` _workersselected _asworker_unit)
        (`KismetSystemLibrary.PrintString` "Added worker to selected")))))

(event `Key|LeftMouseButton`
  (params (Key :type "Key Structure"))
  (:`Pressed`
    (if (`BuildingManager.bIsBuilding` (`self.BuildingManager`))
      (`BuildingManager.Build` (`self.BuildingManager`)))))

(event `Key|Escape`
  (params (Key :type "Key Structure"))
  (:`Pressed`
    (if (`BuildingManager.bIsBuilding` (`self.BuildingManager`)) :!label _label
      (`BuildingManager.StopPlacing` (`self.BuildingManager`)))))

(event `Key|BackSpace`
  (params (Key :type "Key Structure"))
  (:`Pressed`
    (goto _label)))

(fn `UserConstructionScript`)