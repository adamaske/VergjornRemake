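; HUD Blueprint that draws a mouse-drag selection box on screen.
; StartSelection stores the mouse position as the first corner and turns drawing on, and StopSelection turns it off.
; While drawing, DrawHUD updates the second corner from the mouse each frame and draws a translucent cyan rectangle.
; It also queries all Actors inside that rectangle every frame, but does nothing further with the result.
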(event `self.ReceiveTick`
  (params (DeltaSeconds :type "Float (single-precision)")))

(event `/Game/Blueprints/SelectionInterface.StartSelection`
  (bind (_locationx _locationy) (`PlayerController.GetMousePosition` (`GameplayStatics.GetPlayerController` 0)))
  (set `self.SelectionPointA` (`KismetMathLibrary.MakeVector2D` _locationx _locationy))
  (set `self.IsDrawing` true))

(event `self.ReceiveDrawHUD`
  (params (SizeX :type Integer) (SizeY :type Integer))
  (bind (_selectionpointa_x _selectionpointa_y) (`KismetMathLibrary.BreakVector2D` (`self.SelectionPointA`)))
  (bind (_selectionpointb_x _selectionpointb_y) (`KismetMathLibrary.BreakVector2D` (`self.SelectionPointB`)))
  (bind (_locationx _locationy) (`PlayerController.GetMousePosition` (`GameplayStatics.GetPlayerController` 0)))
  (if (`self.IsDrawing`)
    (set `self.SelectionPointB` (`KismetMathLibrary.MakeVector2D` _locationx _locationy))
    (`self.DrawRect` (struct :`R` 0.102654 :`G` 1.0 :`B` 0.950236 :`A` 0.195) _selectionpointa_x _selectionpointa_y (- _selectionpointb_x _selectionpointa_x) (- _selectionpointb_y _selectionpointa_y))
    (set `self.Out Actors` (`self.GetActorsInSelectionRectangle` "/Script/Engine.Actor" (`self.SelectionPointA`) (`self.SelectionPointB`)))))

(event `/Game/Blueprints/SelectionInterface.StopSelection`
  (set `self.IsDrawing` false))

(fn `UserConstructionScript`)