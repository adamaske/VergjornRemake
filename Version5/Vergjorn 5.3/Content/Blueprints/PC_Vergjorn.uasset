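; Player controller that detects whether the player is using gamepad or keyboard and mouse.
; Key presses update the stored input type and call SwitchInputMode only on a device change, and a debug listener prints InputTypeSwitched notifications.
; A SetInputMode helper applies UI-only mode, which requires a valid widget but does not focus it, or Game-and-UI mode, which always shows the cursor.
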(event `InputAction|KeyDetect`
  (params (Key :type "Key Structure"))
  ;[1 1 1] Input
  ;;[1 1 1] Input Switcher
  (:`Pressed`
    (if (`KismetInputLibrary.Key_IsGamepadKey` Key)
      (switch `E_V_InputType` (`self.m_InputType`)
        (:`IT_KeyboardMouse`
          (set `self.m_InputType` "IT_Gamepad")
          (`self.SwitchInputMode` (`self.m_InputType`) :!label _label)))
      (elif (or (`KismetInputLibrary.Key_IsKeyboardKey` Key) (`KismetInputLibrary.Key_IsMouseButton` Key))
        (switch `E_V_InputType` (`self.m_InputType`)
          (:`IT_Gamepad`
            (set `self.m_InputType` "IT_KeyboardMouse")
            (goto _label)))))))

(event `InputTypeSwitched_Event`
  (params (new_type :type "E_V_InputType Enum" :default "IT_KeyboardMouse"))
  ;[1 1 1] Input
  ;;[1 1 1] Debug Input Type Switched
  (`KismetSystemLibrary.PrintString` (`KismetStringLibrary.Concat_StrStr` "Set InputType : " (`|GetEnumeratorNameAsString` new_type)) true true (struct :`R` 0.053399 :`G` 1.0 :`A` 1.0) 5.0))

(event `self.ReceiveBeginPlay`
  (`|ExecutionSequence`
    (:`then_0`
      ;[1 1 1] Input
      ;;[1 1 1] Debug Input Type Switched
      (add `self.m_InputTypeSwitched` self (delegate `InputTypeSwitched_Event`)))))

(fn `SetInputMode`
  (params (ShowMouse :type Boolean) (UIOnly :type Boolean) (FocusedWidget :type "UserWidget Object Reference"))
  (`|ExecutionSequence`
    (:`then_0`
      (set `self.bShowMouseCursor` ShowMouse))
    (:`then_1`
      (if UIOnly
        (`/Engine/EditorBlueprintResources/StandardMacros.IsValid` FocusedWidget
          (:`Is Valid`
            (`WidgetBlueprintLibrary.SetInputMode_UIOnlyEx` self null "DoNotLock" true))
          (:`Is Not Valid`
            (`KismetSystemLibrary.PrintString` (`KismetStringLibrary.Concat_StrStr` "No Widget Focus") true true (struct :`R` 1.0 :`G` 0.008526 :`A` 1.0) 5.0)))
        (else
          (`/Engine/EditorBlueprintResources/StandardMacros.IsValid` FocusedWidget
            (:`Is Valid`
              (`WidgetBlueprintLibrary.SetInputMode_GameAndUIEx` self FocusedWidget "DoNotLock" false true))
            (:`Is Not Valid`
              (`WidgetBlueprintLibrary.SetInputMode_GameAndUIEx` self null "DoNotLock" false true)))
          (set `self.bShowMouseCursor` true))))))

(fn `UserConstructionScript`)