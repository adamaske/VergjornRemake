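; Blueprint function library giving global shortcuts to the Vergjorn game's core framework objects.
; Three getters fetch the game instance, game mode and first local player controller, each cast to its Vergjorn subclass.
; A failed cast ends the function without returning a valid reference.
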(fn `Get Vergjorn GI`
  (returns (GI :type "/Game/Blueprints/GI_Vergjorn Object Reference"))
  (bind _asgi_vergjorn (cast `/Game/Blueprints/GI_Vergjorn` (`GameplayStatics.GetGameInstance` null)))
  (return _asgi_vergjorn))

(fn `Get Vergjorn GM`
  (returns (GM :type "/Game/Blueprints/GM_Vergjorn Object Reference"))
  (bind _asgm_vergjorn (cast `/Game/Blueprints/GM_Vergjorn` (`GameplayStatics.GetGameMode` null)))
  (return _asgm_vergjorn))

(fn `Get Vergjorn PC`
  (returns (PC :type "/Game/Blueprints/PC_Vergjorn Object Reference"))
  (bind _aspc_vergjorn (cast `/Game/Blueprints/PC_Vergjorn` (`GameplayStatics.GetPlayerController` null)))
  (return _aspc_vergjorn))